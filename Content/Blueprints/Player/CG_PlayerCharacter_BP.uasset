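; CG_PlayerCharacter_BP is the player character Blueprint that owns the player HUD and handles cursor and viewport focus.
; On BeginPlay it creates CG_PlayerHUD_WBP and adds it to the player screen.
; Events switch the cursor between grab and open hand for dragging, return input to game-only with viewport focus, and show the HUD only in the default state, hiding it while inspecting, in inventory or paused.
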(event EventBeginPlay
  (bind _returnvalue (UserInterface|CreateWidget "/Game/Blueprints/Widgets/CG_PlayerHUD_WBP.CG_PlayerHUD_WBP_C" (Game|GetPlayerController 0)))
  (Variables|Default|SetHUD _returnvalue)
  (UserInterface|Viewport|AddtoPlayerScreen _returnvalue))

(event EventChangeHUD
  (params (curState :type EPlayerState%20Enum :default "DEFAULT"))
  (bind _hud (Variables|Default|GetHUD))
  (switch Utilities|FlowControl|Switch|SwitchonEPlayerState curState
    (:DEFAULT
      (Widget|SetVisibility _hud "Visible"))
    (:INSPECTING
      (Widget|SetVisibility _hud "Hidden" :!label _label))
    (:INVENTORY
      (goto _label))
    (:PAUSED
      (goto _label))))

(event EventUpdateCursor
  (params (isDragging :type Boolean))
  (if isDragging
    (Variables|/Script/Engine.PlayerController|SetCurrentMouseCursor (Game|GetPlayerController 0) "GrabHand")
    (else
      (Variables|/Script/Engine.PlayerController|SetCurrentMouseCursor (Game|GetPlayerController 0) "Hand"))))

(event EventFocusViewport
  (Input|SetInputModeGameOnly (Game|GetPlayerController 0))
  (Class|WidgetBlueprintLibrary|SetFocustoGameViewport))

(fn ConstructionScript)